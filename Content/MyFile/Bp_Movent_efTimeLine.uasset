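; Demo-style movement actor that slides its Cube back and forth along relative X while spinning it in yaw.
; From BeginPlay, a direction flag chooses whether the timeline plays forward or in reverse.
; Each timeline update scales the track value into the X position and adds a fixed rotation step.
; On finish, the flag flips and re-enters the branch for an endless ping-pong; the Play function sets the flag.
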(event `self.ReceiveBeginPlay`
  (bind _cube (`self.Cube`))
  (if (`self.방향설정1`) :!label _label
    (bind (_direction `_새_트랙_0`) (`Timeline|타임라인_0` :!label _label_2)
      (:`Update`
        (`SceneComponent.K2_SetRelativeLocation` _cube (`KismetMathLibrary.MakeVector` (* 500 `_새_트랙_0`)) false false)
        (`SceneComponent.K2_AddLocalRotation` _cube (`KismetMathLibrary.MakeRotator` 0.0 0.0 10.0) false false))
      (:`Finished`
        (set `self.방향설정1` (not (`self.방향설정1`)))
        (goto _label)))
    (else
      (goto _label_2 :!via `Reverse`))))

(fn `Play`
  (params (playup :type Boolean))
  (set `self.방향설정1` playup))

(fn `UserConstructionScript`)