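; Actor Blueprint that slides its Cube component back and forth along the relative X axis, like a simple oscillating mover.
; While the Right flag is set, Tick offsets the cube by a fixed, frame-rate-dependent step without sweep.
; IsMoveRit holds the direction and flips when the cube reaches Endpoint or returns to zero.
; The Play function sets Right to start or stop the motion.
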(event `self.ReceiveTick`
  (params (DeltaSeconds :type "Float (single-precision)"))
  (bind _cube (`self.Cube`))
  (bind _cube_2 (`self.Cube`))
  (bind _relativelocation_x (`KismetMathLibrary.BreakVector` (`SceneComponent.RelativeLocation` _cube)))
  (bind _relativelocation_x_2 (`KismetMathLibrary.BreakVector` (`SceneComponent.RelativeLocation` _cube_2)))
  (if (`self.right`)
    (if (`self.IsMoveRit`)
      (`SceneComponent.K2_AddRelativeLocation` _cube_2 (5.0 0.0 0.0) false false)
      (if (>= _relativelocation_x_2 (`self.Endpoint`))
        (set `self.IsMoveRit` false))
      (else
        (`SceneComponent.K2_AddRelativeLocation` _cube (-5.0 0.0 0.0) false false)
        (if (<= _relativelocation_x 0.0)
          (set `self.IsMoveRit` true))))))

(fn `play`
  (params (right :type Boolean))
  (set `self.right` right))

(fn `UserConstructionScript`)