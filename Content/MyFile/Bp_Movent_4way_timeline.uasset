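; Actor Blueprint that moves a Cube around a looping square path, started and paused through the third-person character's F-key dispatcher or a Play function.
; One timeline, scaled by Metric, drives relative X or Y by the current direction, playing forward for Right/Up and backward for Left/Down.
; Each finish advances the direction and starts the next leg.
; Stopping stores the play direction in Playtype, so movement resumes mid-leg.
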(event `Play event`
  (switch `/Game/MyFile/4way_timelineplayset` (`self.playtype`)
    (:`NewEnumerator0`
      (switch `/Game/MyFile/En_Move_Tipe` (`self.4waytype`) :!label _label
        (:`NewEnumerator0`
          (bind (_direction `_새_트랙_0`) (`Timeline|타임라인_0` :!via `PlayFromStart` :!label _label_2)
            (:`Update`
              (`self.NewFunction_0` `_새_트랙_0`))
            (:`Finished`
              (`self.NewFunction_1`)
              (goto _label))))
        (:`NewEnumerator1`
          (goto _label_2 :!via `PlayFromStart`))
        (:`NewEnumerator2`
          (goto _label_2 :!via `ReverseFromEnd`))
        (:`NewEnumerator3`
          (goto _label_2 :!via `ReverseFromEnd`))))
    (:`NewEnumerator1`
      (goto _label_2))
    (:`NewEnumerator2`
      (goto _label_2 :!via `Reverse`))))

(event `stop`
  (`self.NewFunction_2`)
  (goto _label_2 :!via `Stop`))

(event `self.ReceiveBeginPlay`
  (bind _asthird_person_character (cast `/Game/ThirdPersonBP/Blueprints/ThirdPersonCharacter` (`GameplayStatics.GetPlayerCharacter` 0)))
  (add `/Game/ThirdPersonBP/Blueprints/ThirdPersonCharacter.EventDispatcher_F_Key` _asthird_person_character (`|CreateDelegate` :!event `Bp_Movent_4way_timeline_AutoGenFunc`)))

(fn `Bp_Movent_4way_timeline_AutoGenFunc`
  (params (IsPressed :type Boolean))
  (if IsPressed
    (`self.Play event`)
    (else
      (`self.stop`))))

(fn `NewFunction_0`
  (params (value :type "Float (double-precision)"))
  (bind _cube (`self.Cube`))
  (bind _returnvalue (* value (`self.metric`)))
  (bind (_relativelocation_x _relativelocation_y) (`KismetMathLibrary.BreakVector` (`SceneComponent.RelativeLocation` _cube)))
  (switch `/Game/MyFile/En_Move_Tipe` (`self.4waytype`)
    (:`NewEnumerator0`
      (`SceneComponent.K2_SetRelativeLocation` _cube (`KismetMathLibrary.MakeVector` _returnvalue _relativelocation_y) false false :!label _label))
    (:`NewEnumerator1`
      (`SceneComponent.K2_SetRelativeLocation` _cube (`KismetMathLibrary.MakeVector` _relativelocation_x _returnvalue) false false :!label _label_2))
    (:`NewEnumerator2`
      (goto _label))
    (:`NewEnumerator3`
      (goto _label_2))))

(fn `NewFunction_1`
  (switch `/Game/MyFile/En_Move_Tipe` (`self.4waytype`)
    (:`NewEnumerator0`
      (set `self.4waytype` "NewEnumerator1"))
    (:`NewEnumerator1`
      (set `self.4waytype` "NewEnumerator2"))
    (:`NewEnumerator2`
      (set `self.4waytype` "NewEnumerator3"))
    (:`NewEnumerator3`
      (set `self.4waytype` "NewEnumerator0")))
  (return))

(fn `NewFunction_2`
  (switch `/Game/MyFile/En_Move_Tipe` (`self.4waytype`)
    (:`NewEnumerator0`
      (set `self.playtype` "NewEnumerator1" :!label _label))
    (:`NewEnumerator1`
      (goto _label))
    (:`NewEnumerator2`
      (set `self.playtype` "NewEnumerator2" :!label _label_2))
    (:`NewEnumerator3`
      (goto _label_2))))

(fn `play`
  (params (input :type Boolean))
  (returns (Result :type Boolean))
  (if input
    (`self.Play event`)
    (else
      (`self.stop`)))
  (return true))

(fn `UserConstructionScript`)