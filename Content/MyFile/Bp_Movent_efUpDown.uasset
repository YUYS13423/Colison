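; Cube platform actor that oscillates vertically between relative Z zero and Endpoint while its Playup flag is set.
; BeginPlay binds to the ThirdPersonCharacter's FKey dispatcher, with a generated handler that copies the pressed state into Playup.
; Tick moves the cube a fixed step per frame without sweep or delta-time scaling, flipping IsMoveRit at each limit.
; The rotation step is zero, and the Play setter's only graph call is unconnected.
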(event `self.ReceiveTick`
  (params (DeltaSeconds :type "Float (single-precision)"))
  (bind _cube (`self.Cube`))
  (bind _cube_2 (`self.Cube`))
  (bind (_relativelocation_x _relativelocation_y _relativelocation_z) (`KismetMathLibrary.BreakVector` (`SceneComponent.RelativeLocation` _cube)))
  (bind (_relativelocation_x_2 _relativelocation_y_2 _relativelocation_z_2) (`KismetMathLibrary.BreakVector` (`SceneComponent.RelativeLocation` _cube_2)))
  (if (`self.playup`)
    (`SceneComponent.K2_AddRelativeRotation` :`self` _cube_2)
    (if (`self.IsMoveRit`)
      (`SceneComponent.K2_AddRelativeLocation` _cube_2 (0.0 0.0 5.0) false false)
      (if (>= _relativelocation_z_2 (`self.Endpoint`))
        (set `self.IsMoveRit` false))
      (else
        (`SceneComponent.K2_AddRelativeLocation` _cube (0.0 0.0 -5.0) false false)
        (if (<= _relativelocation_z 0.0)
          (set `self.IsMoveRit` true))))))

(event `self.ReceiveBeginPlay`
  (bind _asthird_person_character (cast `/Game/ThirdPersonBP/Blueprints/ThirdPersonCharacter` (`GameplayStatics.GetPlayerCharacter` 0)))
  (add `/Game/ThirdPersonBP/Blueprints/ThirdPersonCharacter.EventDispatcher_F_Key` _asthird_person_character (`|CreateDelegate` :!event `Bp_Movent_efUpDown_AutoGenFunc`)))

(fn `Bp_Movent_efUpDown_AutoGenFunc`
  (params (IsPressed :type Boolean))
  (set `self.playup` IsPressed))

(fn `play`
  (params (input :type Boolean))
  (returns (Result :type Boolean))
  (set `self.playup` input)
  (return true))

(fn `UserConstructionScript`)