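; Blueprint actor that moves its Cube component around a looping square path in the local XY plane.
; Each Tick switches on a four-state direction enum and offsets the cube by Sp along the matching axis.
; When the relative location passes Endpoint or returns to zero, the enum advances from Right to Up, Left, Down and back to Right.
; Speed is applied per frame without delta time scaling, so movement depends on frame rate.
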(event `self.ReceiveTick`
  (params (DeltaSeconds :type "Float (single-precision)"))
  (bind _endpoint (`self.Endpoint`))
  (bind _cube (`self.Cube`))
  (bind _sp (`self.sp`))
  (bind _cube_2 (`self.Cube`))
  (bind _returnvalue (* -1 _sp))
  (bind (_relativelocation_x _relativelocation_y) (`KismetMathLibrary.BreakVector` (`SceneComponent.RelativeLocation` (`self.Cube`))))
  (switch `/Game/MyFile/En_Move_Tipe` (`self.4waytype`)
    (:`NewEnumerator0`
      (`SceneComponent.K2_AddLocalOffset` _cube (`KismetMathLibrary.MakeVector` _sp) false false)
      (if (>= _relativelocation_x _endpoint)
        (set `self.4waytype` "NewEnumerator1")))
    (:`NewEnumerator1`
      (`SceneComponent.K2_AddLocalOffset` _cube (`KismetMathLibrary.MakeVector` 0.0 _sp) false false)
      (if (>= _relativelocation_y _endpoint)
        (set `self.4waytype` "NewEnumerator2")))
    (:`NewEnumerator2`
      (`SceneComponent.K2_AddLocalOffset` _cube_2 (`KismetMathLibrary.MakeVector` _returnvalue) false false)
      (if (>= 0.0 _relativelocation_x)
        (set `self.4waytype` "NewEnumerator3")))
    (:`NewEnumerator3`
      (`SceneComponent.K2_AddLocalOffset` _cube_2 (`KismetMathLibrary.MakeVector` 0.0 _returnvalue) false false)
      (if (>= 0.0 _relativelocation_y)
        (set `self.4waytype` "NewEnumerator0")))))

(fn `UserConstructionScript`)